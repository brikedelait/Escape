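; Level exit trigger that finishes the match when a BP_TopDownCharacter overlaps its box and records the Min : Sec time from BP_TopDownGameMode.
; Without an AdministratorComponent actor, it sends a win notification through the first PlayerComponent.
; Otherwise, the administrator sends the time with its local IP, counts finishers and flags when all connected players are done.
; Both paths update and show the WinMenu, reveal the cursor and pause.
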(event `self.Box.OnComponentBeginOverlap`
  (params (OverlappedComponent :type "PrimitiveComponent Object Reference") (OtherActor :type "Actor Object Reference") (OtherComp :type "PrimitiveComponent Object Reference") (OtherBodyIndex :type Integer) (bFromSweep :type Boolean) (SweepResult :type "HitResult Structure (by ref)"))
  (cast `/Game/TopDown/Blueprints/BP_TopDownCharacter` OtherActor)
  (bind _outactors (`GameplayStatics.GetAllActorsOfClass` "/Game/ThirdPersonBP/AdministratorComponent.AdministratorComponent_C"))
  (if (`KismetArrayLibrary.Array_IsEmpty` _outactors)
    (bind _outactors_2 (`GameplayStatics.GetAllActorsOfClass` "/Game/ThirdPersonBP/PlayerComponent.PlayerComponent_C"))
    (bind _output (`|GetArrayItem` _outactors_2))
    (`/Game/ThirdPersonBP/PlayerComponent.SendWinMatchNotification` _output)
    (bind _asbp_top_down_game_mode (cast `/Game/TopDown/Blueprints/BP_TopDownGameMode` (`GameplayStatics.GetGameMode`)))
    (bind _result (`|FormatText` "{Min} : {Sec}" (`/Game/TopDown/Blueprints/BP_TopDownGameMode.TimeMin` _asbp_top_down_game_mode) (`/Game/TopDown/Blueprints/BP_TopDownGameMode.TimeSec` _asbp_top_down_game_mode)))
    (bind _returnvalue (`KismetArrayLibrary.Array_Add` (`/Game/ThirdPersonBP/PlayerComponent.ChronoPlayers` _output) _result))
    (bind _result_2 (`/Engine/EditorBlueprintResources/StandardMacros.IncrementInt` _returnvalue)
      (:`  `
        (bind _winmenu (`/Game/ThirdPersonBP/PlayerComponent.WinMenu` _output))
        (`/Game/Menu/Win_Menu.OnNewPlayerFinished` _winmenu _result_2 _result)
        (`UserWidget.AddToViewport` _winmenu 0)
        (set `PlayerController.bShowMouseCursor` true (`GameplayStatics.GetPlayerController` 0))
        (`GameplayStatics.SetGamePaused` true)))
    (else
      (bind _asbp_top_down_game_mode_2 (cast `/Game/TopDown/Blueprints/BP_TopDownGameMode` (`GameplayStatics.GetGameMode`)))
      (bind _output_2 (`|GetArrayItem` _outactors))
      (bind _result_3 (`|FormatText` "{Min} : {Sec}" (`/Game/TopDown/Blueprints/BP_TopDownGameMode.TimeMin` _asbp_top_down_game_mode_2) (`/Game/TopDown/Blueprints/BP_TopDownGameMode.TimeSec` _asbp_top_down_game_mode_2)))
      (bind _returnvalue_2 (`KismetArrayLibrary.Array_Add` (`/Game/ThirdPersonBP/AdministratorComponent.ChronoPlayers` _output_2) _result_3))
      (bind _result_4 (`/Engine/EditorBlueprintResources/StandardMacros.IncrementInt` _returnvalue_2)
        (:`  `
          (bind _winmenu_2 (`/Game/ThirdPersonBP/AdministratorComponent.WinMenu` _output_2))
          (`/Game/Menu/Win_Menu.OnNewPlayerFinished` _winmenu_2 _result_4 _result_3)
          (bind _result_5 (`/Engine/EditorBlueprintResources/StandardMacros.IncrementInt` (`/Game/ThirdPersonBP/AdministratorComponent.PlayerFinished` _output_2))
            (:`  `
              (`/Game/ThirdPersonBP/AdministratorComponent.SendNewPlayerFinished` _output_2 _result_3 (`/Game/ThirdPersonBP/AdministratorComponent.LocalIp` _output_2))
              (if (not (!= _result_5 (`/Game/ThirdPersonBP/AdministratorComponent.PlayersConnected` _output_2)))
                (`/Game/Menu/Win_Menu.OnAllPlayerFinished` _winmenu_2))
              (`UserWidget.AddToViewport` _winmenu_2 0)
              (set `PlayerController.bShowMouseCursor` true (`GameplayStatics.GetPlayerController` 0))
              (`GameplayStatics.SetGamePaused` true))))))))

(fn `UserConstructionScript`)