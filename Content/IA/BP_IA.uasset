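; BP_IA is an enemy AI pawn that chases the player on sight and ends the game upon reaching them.
; PawnSensing triggers a faster AIMoveTo chase on seeing the player or hearing near-zero-volume noises; success shows GameOver, pauses and destroys the pawn.
; A self-repeating Ronde event patrols random reachable points, but nothing here starts it, nor calls Walk to lower speed.
; The mesh loops a walk animation from BeginPlay.
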(event `self.ReceiveBeginPlay`
  (`SkeletalMeshComponent.PlayAnimation` (`self.Mesh`) "/Game/Characters/Mannequins/Animations/Quinn/MF_Walk_Fwd.MF_Walk_Fwd" true))

(event `self.PawnSensing.OnSeePawn`
  (params (Pawn :type "Pawn Object Reference"))
  (if (== Pawn (`GameplayStatics.GetPlayerCharacter` 0))
    (`self.run`)
    (`|AIMoveTo` self (0.0 0.0 0.0) Pawn
      (:`OnSuccess`
        (bind _returnvalue (`|CreateWidget` "/Game/Menu/GameOver.GameOver_C" :!label _label))
        (`UserWidget.AddToViewport` _returnvalue 0)
        (set `PlayerController.bShowMouseCursor` true (`GameplayStatics.GetPlayerController` 0))
        (`GameplayStatics.SetGamePaused` true)
        (`self.K2_DestroyActor`)))))

(event `self.PawnSensing.OnHearNoise`
  (params (Instigator :type "Pawn Object Reference") (Location :type "Vector Structure (by ref)") (Volume :type "Float (single-precision)"))
  (if (`KismetMathLibrary.NearlyEqual_FloatFloat` Volume 0.0 0.01)
    (`self.run`)
    (`|AIMoveTo` self (0.0 0.0 0.0) Instigator
      (:`OnSuccess`
        (goto _label)))))

(event `ronde`
  (`|AIMoveTo` self (`NavigationSystemV1.K2_GetRandomReachablePointInRadius` (`self.K2_GetActorLocation`) 5000.0 null null) null
    (:`OnSuccess`
      _)
    (:`OnFail`
      _))
  (`self.ronde`))

(fn `run`
  (set `CharacterMovementComponent.MaxWalkSpeed` 200.0 (`self.CharacterMovement`)))

(fn `UserConstructionScript`)

(fn `walk`
  (set `CharacterMovementComponent.MaxWalkSpeed` 100.0 (`self.CharacterMovement`)))